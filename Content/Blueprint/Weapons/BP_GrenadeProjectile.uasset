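; Grenade projectile actor that explodes on a fixed fuse timer shortly after it spawns.
; BeginPlay waits out the delay, then Explode spawns an explosion emitter at the sphere component and applies full, non-falloff radial damage credited to the instigator's controller.
; It also draws a debug sphere showing the blast radius, then destroys itself.
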(event `self.ReceiveBeginPlay`
  (`KismetSystemLibrary.Delay` 1.0)
  (`self.Explode`))

(event `Explode`
  (bind _returnvalue (`SceneComponent.K2_GetComponentLocation` (`self.Sphere`)))
  (`GameplayStatics.SpawnEmitterAtLocation` "/Game/WeaponEffects/Explosion/P_Explosion.P_Explosion" _returnvalue)
  (`GameplayStatics.ApplyRadialDamage` :`BaseDamage` 100.0 :`Origin` _returnvalue :`DamageRadius` 200.0 :`DamageCauser` self :`InstigatedByController` (`self.GetInstigatorController`) :`bDoFullDamage` true)
  (`KismetSystemLibrary.DrawDebugSphere` _returnvalue 200.0 12 (struct :`R` 1.0 :`G` 0.01492 :`A` 1.0) 1.0)
  (`self.K2_DestroyActor`))

(fn `UserConstructionScript`)